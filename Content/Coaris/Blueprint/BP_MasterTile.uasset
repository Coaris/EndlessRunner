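; BP_MasterTile is a pooled tube track tile that rotates around its roll axis when the player changes lanes.
; It binds to the player's ChangeLane dispatcher and, while active, uses a timeline to lerp its roll to the target angle.
; Activate and deactivate events toggle mesh collision.
; Player overlap with the box broadcasts OnTileUsed after a short delay for recycling, while the direct ReturnToPool call is left unwired.
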(event `self.ReceiveBeginPlay`
  ;[1 1 1] Get player character
  (bind _asbp_third_person_character (cast `/Game/ThirdPerson/Blueprints/BP_ThirdPersonCharacter` (`GameplayStatics.GetPlayerCharacter` 0)))
  (bind _output_get (set `self.Player` _asbp_third_person_character))
  ;[1 1 1] Change lane
  (add `/Game/ThirdPerson/Blueprints/BP_ThirdPersonCharacter.ChangeLane` _output_get (delegate `ChangeLane_Event`))
  (bind _returnvalue (`GameplayStatics.GetActorOfClass` "/Game/Coaris/Blueprint/BP_TilePool.BP_TilePool_C")))

(event `ChangeLane_Event`
  (params (TargetAngle :type "Float (double-precision)"))
  ;[1 1 1] Change lane
  (if (`self.IsActiving`)
    (set `self.TargetAngle` TargetAngle)
    (bind (_direction _lerp_alpha) (`Timeline|Lerp Timer` :!via `PlayFromStart`)
      (:`Update`
        (`SceneComponent.K2_SetWorldRotation` (`self.Root`) (`KismetMathLibrary.MakeRotator` (`KismetMathLibrary.Lerp` (`self.CurrentAngle`) (`self.TargetAngle`) _lerp_alpha)) false false))
      (:`Finished`
        (set `self.CurrentAngle` (`self.TargetAngle`))))))

(event `ActiveTile`
  (`PrimitiveComponent.SetCollisionEnabled` (`self.SM_TubeTile`) "QueryOnly"))

(event `Deactive Tile`
  (`PrimitiveComponent.SetCollisionEnabled` (`self.SM_TubeTile`) "NoCollision"))

(event `self.Box Collider.OnComponentBeginOverlap`
  (params (OverlappedComponent :type "PrimitiveComponent Object Reference") (OtherActor :type "Actor Object Reference") (OtherComp :type "PrimitiveComponent Object Reference") (OtherBodyIndex :type Integer) (bFromSweep :type Boolean) (SweepResult :type "HitResult Structure (by ref)"))
  (cast `/Game/ThirdPerson/Blueprints/BP_ThirdPersonCharacter` OtherActor)
  (`|ExecutionSequence`
    (:`then_0`
      ;[1 1 1] Put self back to pool delay 1 sec
      (`KismetSystemLibrary.Delay` 1.0)
      (`self.OnTileUsed` self))))

(fn `UserConstructionScript`)