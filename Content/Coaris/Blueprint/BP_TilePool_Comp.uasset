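; BP_TilePool_Comp is a component that pre-spawns a pool of BP_MasterTile actors for its owner.
; On BeginPlay it spawns AmountOfTiles tiles at the owner's location, disables their tube mesh collision and attaches them to the owner.
; Each tile's OnTileUsed dispatcher is bound to ReturnToPool, which teleport-free moves it back to the owner and reattaches it.
; The attached actors serve as the pool, with no array or retrieval logic here.
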(event `self.ReceiveBeginPlay`
  ;[1 1 1] Set up the tile pool array
  (for _ (range (`self.AmountOfTiles`))
    ;[1 1 1] Spawn tiles at the owner location
    (bind _returnvalue (`|SpawnActorFromClass` "/Game/Coaris/Blueprint/BP_MasterTile.BP_MasterTile_C" (`KismetMathLibrary.MakeTransform` (`Actor.K2_GetActorLocation` (`self.GetOwner`))) "Undefined" "MultiplyWithRoot" null null))
    (`PrimitiveComponent.SetCollisionEnabled` (`/Game/Coaris/Blueprint/BP_MasterTile.SM_TubeTile` _returnvalue) "NoCollision")
    (`Actor.K2_AttachToActor` _returnvalue (`self.GetOwner`) "None" "KeepWorld" "KeepWorld" "KeepWorld" true)
    (add `/Game/Coaris/Blueprint/BP_MasterTile.OnTileUsed` _returnvalue (delegate `ReturnToPool`))))

(event `ReturnToPool`
  (params (Tile :type "/Game/Coaris/Blueprint/BP_MasterTile Object Reference"))
  (bind _returnvalue (`self.GetOwner`))
  (`Actor.K2_SetActorLocation` Tile (`Actor.K2_GetActorLocation` _returnvalue) false false)
  (`Actor.K2_AttachToActor` Tile _returnvalue "None" "KeepWorld" "KeepWorld" "KeepWorld" true))